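; Player character Blueprint prototyping touch-drag rotation, with debug output in place of working rotation.
; Touch press and move handlers store finger locations normalised by screen resolution.
; Another move handler crosses the current location with the start location, prints a scaled rotation derived from it, and sets the player's relative rotation to zero.
; The stored previous-frame location feeds only a disconnected debug print, and Tick is empty.
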(event `InputTouch`
  (params (Location :type "Vector Structure") (FingerIndex :type "ETouchIndex Enum"))
  ;[1 1 1] Set finger position at start of touch
  (:`Pressed`
    ;;[1 1 1] Convert raw touch location into vector with value range of 0 to 1 in relation to screen resolution.
    (bind _returnvalue (`GameUserSettings.GetGameUserSettings`))
    (bind (_returnvalue_x _returnvalue_y) (break `IntPoint` (`GameUserSettings.GetScreenResolution` _returnvalue)))
    (set `self.Location From Start of Touch` (`KismetMathLibrary.MakeVector` (/ Location_X (`KismetMathLibrary.Conv_IntToDouble` _returnvalue_x)) (/ Location_Y (`KismetMathLibrary.Conv_IntToDouble` _returnvalue_y)) Location_Z))))

(event `InputTouch`
  (params (Location :type "Vector Structure") (FingerIndex :type "ETouchIndex Enum"))
  ;[1 1 1] Set finger position from previous frame
  (:`Moved`
    ;;[1 1 1] Convert raw touch location into vector with value range of 0 to 1 in relation to screen resolution.
    (bind _returnvalue (`GameUserSettings.GetGameUserSettings`))
    (bind (_returnvalue_x _returnvalue_y) (break `IntPoint` (`GameUserSettings.GetScreenResolution` _returnvalue)))
    (set `self.Location from previous frame` (`KismetMathLibrary.MakeVector` (/ Location_X (`KismetMathLibrary.Conv_IntToDouble` _returnvalue_x)) (/ Location_Y (`KismetMathLibrary.Conv_IntToDouble` _returnvalue_y)) Location_Z))))

(event `self.ReceiveTick`
  (params (DeltaSeconds :type "Float (single-precision)")))

(event `InputTouch`
  (params (Location :type "Vector Structure") (FingerIndex :type "ETouchIndex Enum"))
  (:`Moved`
    ;[1 1 1] Convert raw touch location into vector with value range of 0 to 1 in relation to screen resolution.
    (bind _returnvalue (`GameUserSettings.GetGameUserSettings`))
    (bind (_returnvalue_x _returnvalue_y) (break `IntPoint` (`GameUserSettings.GetScreenResolution` _returnvalue)))
    (`KismetSystemLibrary.PrintString` (`KismetStringLibrary.Conv_RotatorToString` (* (`KismetMathLibrary.Conv_VectorToRotator` (`KismetMathLibrary.Cross_VectorVector` (`KismetMathLibrary.MakeVector` (/ Location_X (`KismetMathLibrary.Conv_IntToDouble` _returnvalue_x)) (/ Location_Y (`KismetMathLibrary.Conv_IntToDouble` _returnvalue_y)) Location_Z) (`self.Location From Start of Touch`))) 0.05)))
    (`self.K2_SetActorRelativeRotation` (`GameplayStatics.GetPlayerCharacter` 0) (`KismetMathLibrary.MakeRotator` 0.0) false false)))

(event `InputTouch`
  (params (Location :type "Vector Structure") (FingerIndex :type "ETouchIndex Enum"))
  ;[1 1 1] Print finger location from previous frame - set input touch from move to enable
)

(event `InputTouch`
  (params (Location :type "Vector Structure") (FingerIndex :type "ETouchIndex Enum"))
  ;[1 1 1] Print finger location at start of touch - set input touch from move to enable
)

(event `InputTouch`
  (params (Location :type "Vector Structure") (FingerIndex :type "ETouchIndex Enum"))
  ;[1 1 1] Print current finger location and finger index - set input touch from move to enable
)

(fn `UserConstructionScript`)
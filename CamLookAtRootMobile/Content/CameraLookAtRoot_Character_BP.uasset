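; Character Blueprint for a motion-controlled camera that uses device gravity to swing around and face the world origin.
; It makes itself the view target on BeginPlay.
; Each tick it eases the camera toward the scaled gravity vector as a world position and interpolates its rotation to look back at the origin.
; An unconnected debug print of the motion sensor readings remains in the graph.
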(event `self.ReceiveBeginPlay`
  (`PlayerController.SetViewTargetWithBlend` (`GameplayStatics.GetPlayerController` 0) self 0.0 "VTBlend_Linear" 0.0 false))

(event `self.ReceiveTick`
  (params (DeltaSeconds :type "Float (single-precision)"))
  (`SceneComponent.K2_SetWorldTransform` (`self.Camera`) (`KismetMathLibrary.MakeTransform` (`KismetMathLibrary.VInterpTo` (`SceneComponent.K2_GetComponentLocation` (`self.Camera`)) (* (`.Gravity` (`PlayerController.GetInputMotionState` (`GameplayStatics.GetPlayerController` 0))) 250) (`GameplayStatics.GetWorldDeltaSeconds`) 25.0) (`KismetMathLibrary.RInterpTo` (`SceneComponent.K2_GetComponentRotation` (`self.Camera`)) (`KismetMathLibrary.FindLookAtRotation` (`SceneComponent.K2_GetComponentLocation` (`self.Camera`)) (0.0 0.0 0.0)) (`GameplayStatics.GetWorldDeltaSeconds`) 75.0)) false true))

(fn `UserConstructionScript`)
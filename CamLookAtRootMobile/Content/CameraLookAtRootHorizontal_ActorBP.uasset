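; Camera actor that takes over player 0's view on BeginPlay and orients its spring arm from device motion input.
; Each tick turns the negated gravity vector into pitch and roll, using the derived yaw as roll with a 90-degree offset, then sets the arm's world rotation.
; The tilt-based yaw update, which filters out a recurring false reading, is disconnected, so the event graph never changes yaw.
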(event `self.ReceiveBeginPlay`
  ;[1 1 1] Set view target to this blueprint's camera
  (`PlayerController.SetViewTargetWithBlend` (`GameplayStatics.GetPlayerController` 0) self 0.0 "VTBlend_Linear" 0.0 false))

(event `self.ReceiveTick`
  (params (DeltaSeconds :type "Float (single-precision)"))
  (bind (_returnvalue_x _returnvalue_y _returnvalue_z) (`KismetMathLibrary.BreakVector` (`self.GetInputVectorAxisValue`)))
  (bind (_returnvalue_roll _returnvalue_pitch _returnvalue_yaw) (`KismetMathLibrary.BreakRotator` (`KismetMathLibrary.Conv_VectorToRotator` (* (`KismetMathLibrary.MakeVector` _returnvalue_x _returnvalue_y _returnvalue_z) -1.0))))
  (`|ExecutionSequence`
    (:`then_0`
      ;[1 1 1] Gravity for Pitch and Roll. Note that Yaw is Roll
      (set `self.Pitch` _returnvalue_pitch)
      (set `self.Roll` _returnvalue_yaw))
    (:`then_1`)
    (:`then_2`
      ;[1 1 1] Set World Rotation for Spring Arm
      (`SceneComponent.K2_SetWorldRotation` (`self.SpringArm`) (`KismetMathLibrary.MakeRotator` (+ (`self.Roll`) 90.0) (`self.Pitch`) (`self.Yaw`)) false false))))

(fn `Print String + Input Value`
  (params (`Enable printing` :type Boolean :default true) (String :type String) (`Input Value` :type String))
  (if `Enable printing`
    (`KismetSystemLibrary.PrintString` (`KismetStringLibrary.Concat_StrStr` String `Input Value`))))

(fn `UserConstructionScript`)
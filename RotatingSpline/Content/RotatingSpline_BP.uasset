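; Spline actor that builds a mesh along its spline and, when SpinSpline is on, moves its Scene component along that path.
; The construction script optionally closes the loop and adds a spline mesh component per segment using the configured static mesh.
; Tick advances distance by a speed multiplier, without wrapping, and applies the spline's location and rotation to Scene.
; Several disconnected experiments for orbiting or moving the actor never run.
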(event `self.ReceiveTick`
  (params (DeltaSeconds :type "Float (single-precision)"))
  (if (`self.Spin Spline?`)
    (bind _output_get (set `self.Distance along spline` (+ (`self.Distance along spline`) (* DeltaSeconds (`self.Rotation Speed Multiplier`)))))
    (bind (_returnvalue_location _returnvalue_rotation) (`KismetMathLibrary.BreakTransform` (`SplineComponent.GetTransformAtDistanceAlongSpline` (`self.Spline`) _output_get "World" false)))
    (`SceneComponent.K2_SetWorldLocationAndRotation` (`self.Scene`) _returnvalue_location _returnvalue_rotation false false)))

(fn `UserConstructionScript`
  (bind _closeloopspline (`self.CloseLoopSpline`))
  ;[1 1 1] If closed loop, close loop.
  (`SplineComponent.SetClosedLoop` (`self.Spline`) _closeloopspline _closeloopspline)
  (for _index (range (+ (- (`SplineComponent.GetNumberOfSplinePoints` (`self.Spline`)) (select `bool` (`self.CloseLoopSpline`) :`false` 2 :`true` 1)) 1))
    (bind _returnvalue (`AddComponent|NODE_AddSplineMeshComponent-0` :`bManualAttachment` true))
    (`SceneComponent.K2_AttachToComponent` _returnvalue (`self.Root`) "None" "KeepRelative" "KeepRelative" "KeepRelative" true)
    (bind (_location _tangent) (`SplineComponent.GetLocationAndTangentAtSplinePoint` (`self.Spline`) _index "Local"))
    (bind (_location_2 _tangent_2) (`SplineComponent.GetLocationAndTangentAtSplinePoint` (`self.Spline`) (+ _index 1) "Local"))
    (`SplineMeshComponent.SetStartAndEnd` _returnvalue _location _tangent _location_2 _tangent_2 true)
    (`StaticMeshComponent.SetStaticMesh` _returnvalue (`self.Static Mesh for Spline`))))
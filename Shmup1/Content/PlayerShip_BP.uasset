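; Touch-controlled player ship pawn that follows the finger and auto-fires while the screen is touched.
; Touch press and release toggle IsFiring, which gates both shooting and movement on Tick.
; Shots spawn Projectile_BP at the Arrow and push its mesh forward, using the projectile's own speed and fire rate through a DoOnce-Delay cooldown.
; Movement lerps toward the touch trace's XY hit, or toward LastActorLocation when released.
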(event `self.ReceiveTick`
  (params (DeltaSeconds :type "Float (single-precision)"))
  (bind (_last_actor_location_x _last_actor_location_y) (`KismetMathLibrary.BreakVector` (`self.Last Actor Location`)))
  (bind _returnvalue (`KismetMathLibrary.VLerp` (`self.K2_GetActorLocation`) (`KismetMathLibrary.MakeVector` _last_actor_location_x _last_actor_location_y) 0.5))
  (bind _hitresult (`PlayerController.GetHitResultUnderFingerByChannel` (`GameplayStatics.GetPlayerController` 0) "Touch1" "TraceTypeQuery1" true))
  (bind _returnvalue_2 (`KismetMathLibrary.VLerp` (`self.K2_GetActorLocation`) (`KismetMathLibrary.MakeVector` (.x (`.Location` (`GameplayStatics.BreakHitResult` _hitresult))) (.y (`.Location` (`GameplayStatics.BreakHitResult` _hitresult)))) 0.1))
  (`|ExecutionSequence`
    (:`then_0`
      ;[1 1 1] Fire
      (if (`self.IsFiring?`)
        (`/Engine/EditorBlueprintResources/StandardMacros.DoOnce` false :!label _label
          (:`Completed`
            (`|ExecutionSequence`
              (:`then_0`
                (bind _returnvalue_3 (`|SpawnActorFromClass` "/Game/Projectile_BP.Projectile_BP_C" (`SceneComponent.K2_GetComponentToWorld` (`self.Arrow`)) "AlwaysSpawn" "OverrideRootScale" null null))
                (`PrimitiveComponent.AddForce` (`/Game/Projectile_BP.StaticMesh` _returnvalue_3) (* (`SceneComponent.GetForwardVector` (`self.Arrow`)) (`/Game/Projectile_BP.Projectile Speed` _returnvalue_3)) "None" false)
                (set `self.Fire rate` (`/Game/Projectile_BP.Fire Rate` _returnvalue_3)))
              (:`then_1`
                (`KismetSystemLibrary.Delay` (`self.Fire rate`))
                (goto _label :!via `Reset`)))))))
    (:`then_1`
      (if (`self.IsFiring?`)
        (`self.K2_SetActorLocation` _returnvalue_2)
        (set `self.Last Actor Location` _returnvalue_2)
        (else
          (`self.K2_SetActorLocation` _returnvalue)
          (set `self.Last Actor Location` _returnvalue))))))

(event `InputTouch`
  (params (Location :type "Vector Structure") (FingerIndex :type "ETouchIndex Enum"))
  (:`Pressed`
    (`|ExecutionSequence`
      (:`then_0`
        (set `self.IsFiring?` true))))
  (:`Released`
    (`|ExecutionSequence`
      (:`then_0`
        (set `self.IsFiring?` false)))))

(fn `UserConstructionScript`)
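; Character Blueprint that, judging by its name, provides a camera looking at its root, oriented by a vector passed to its Gravity event.
; Gravity points the spring arm's X axis along the negated vector in world space, with a debug print helper left disabled.
; BeginPlay makes the character the first player's view target and zeroes its movement gravity scale.
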(event `InputVectorAxis|Gravity`
  (params (AxisValue :type "Vector Structure"))
  (bind _returnvalue (`KismetMathLibrary.Conv_VectorToRotator` (* AxisValue -1.0)))
  (`SceneComponent.K2_SetWorldRotation` (`self.SpringArm`) _returnvalue false false)
  (`self.Print String + Input Value` false "axis value" (`KismetStringLibrary.Conv_RotatorToString` _returnvalue)))

(event `self.ReceiveBeginPlay`
  ;[1 1 1] Set view target to this blueprint's camera
  (`PlayerController.SetViewTargetWithBlend` (`GameplayStatics.GetPlayerController` 0) self 0.0 "VTBlend_Linear" 0.0 false)
  (set `CharacterMovementComponent.GravityScale` 0.0 (`self.CharacterMovement`)))

(fn `Print String + Input Value`
  (params (`Enable printing` :type Boolean :default true) (String :type String) (`Input Value` :type String))
  (if `Enable printing`
    (`KismetSystemLibrary.PrintString` (`KismetStringLibrary.Concat_StrStr` String `Input Value`))))

(fn `UserConstructionScript`)
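; Test pawn that takes over the first player controller's view on BeginPlay and forwards touch input to its TouchActorComponentBP.
; Touch press and release events pass location and finger index straight to the component.
; Rotate, pinch and flick axis mappings feed their values into matching component functions, so the pawn only relays input and holds no gesture logic of its own.
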(event `self.ReceiveBeginPlay`
  (`PlayerController.SetViewTargetWithBlend` (`GameplayStatics.GetPlayerController` 0) self 0.0 "VTBlend_Linear" 0.0 false))

(event `InputTouch`
  (params (Location :type "Vector Structure") (FingerIndex :type "ETouchIndex Enum"))
  ;[1 1 1] Must connect these to component
  (:`Pressed`
    (`/Game/CameraTouchControl_ActorComponent_BP.Input Touch Pressed` (`self.TouchActorComponent_BP`) Location FingerIndex))
  (:`Released`
    (`/Game/CameraTouchControl_ActorComponent_BP.Input Touch Released` (`self.TouchActorComponent_BP`) Location FingerIndex)))

(event `InputAxis|RotateAxisMapping`
  (params (AxisValue :type "Float (single-precision)"))
  ;[1 1 1] Must connect these to component
  (`/Game/CameraTouchControl_ActorComponent_BP.Rotate Component` (`self.TouchActorComponent_BP`) AxisValue))

(event `InputAxis|PinchAxisMapping`
  (params (AxisValue :type "Float (single-precision)"))
  ;[1 1 1] Must connect these to component
  (`/Game/CameraTouchControl_ActorComponent_BP.Pinch Component` (`self.TouchActorComponent_BP`) AxisValue))

(event `InputAxis|FlickAxisMapping`
  (params (AxisValue :type "Float (single-precision)"))
  ;[1 1 1] Must connect these to component
  (`/Game/CameraTouchControl_ActorComponent_BP.Flick Component` (`self.TouchActorComponent_BP`) AxisValue))

(fn `UserConstructionScript`)
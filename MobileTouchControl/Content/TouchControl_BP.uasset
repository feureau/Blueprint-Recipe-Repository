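; Touch gesture test Blueprint that becomes player 0's view target on BeginPlay and prints rotate, pinch and flick input for debugging.
; A touch on finger index 1 sets a multi-touch flag that gates per-frame rotate and pinch deltas, derived from current minus previous axis values.
; Flick prints its raw axis value ungated.
; Spring arm length and flick direction logic are unconnected, so no gesture moves the camera.
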(event `self.ReceiveBeginPlay`
  (`PlayerController.SetViewTargetWithBlend` (`GameplayStatics.GetPlayerController` 0) self 0.0 "VTBlend_Linear" 0.0 false))

(event `InputTouch`
  (params (Location :type "Vector Structure") (FingerIndex :type "ETouchIndex Enum")))

(event `InputTouch`
  (params (Location :type "Vector Structure") (FingerIndex :type "ETouchIndex Enum"))
  (:`Pressed`
    (if (== FingerIndex 1)
      (set `self.MultiTouching` true)))
  (:`Released`
    (if (== FingerIndex 1)
      (set `self.MultiTouching` false))))

(event `InputAxis|RotateAxisMapping`
  (params (AxisValue :type "Float (single-precision)"))
  ;[1 1 1] Rotate
  (if (`self.MultiTouching`)
    (bind _output_get (set `self.Rotate Axis mapping Current Frame` AxisValue))
    (bind _output_get_2 (set `self.Rotation Delta` (- _output_get (`self.Rotate Axis mapping Previous Frame`))))
    (`self.Label + input value` "DeltaRotate" (`KismetStringLibrary.Conv_DoubleToString` _output_get_2))
    (set `self.Rotate Axis mapping Previous Frame` (`self.Rotate Axis mapping Current Frame`))
    (else
      (bind _output_get_3 (set `self.Rotate Axis mapping Current Frame` 0.0)))))

(event `InputAxis|PinchAxisMapping`
  (params (AxisValue :type "Float (single-precision)"))
  ;[1 1 1] Pinch
  (if (`self.MultiTouching`)
    (bind _output_get (set `self.Pinch Axis mapping Current Frame` AxisValue))
    (bind _output_get_2 (set `self.PinchDelta` (- _output_get (`self.Pinch Axis mapping Previous Frame`))))
    (`self.Label + input value` "DeltaPinch" (`KismetStringLibrary.Conv_DoubleToString` _output_get_2))
    (set `self.Pinch Axis mapping Previous Frame` (`self.Pinch Axis mapping Current Frame`))
    (else
      (bind _output_get_3 (set `self.Pinch Axis mapping Current Frame` 0.0)))))

(event `InputAxis|FlickAxisMapping`
  (params (AxisValue :type "Float (single-precision)"))
  (`self.Label + input value` "flick" (`KismetStringLibrary.Conv_DoubleToString` AxisValue)))

(fn `Label + input value`
  (params (Label :type String) (`Input Value` :type String))
  (`KismetSystemLibrary.PrintString` (`KismetStringLibrary.Concat_StrStr` Label `Input Value`)))

(fn `UserConstructionScript`)
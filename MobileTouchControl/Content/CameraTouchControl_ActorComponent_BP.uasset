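; Actor component for touch camera control that rotates and zooms the owning actor's SpringArm, fed by touch events and gesture axes.
; A second-finger press snapshots arm rotation and length; rotate interpolates roll and pinch scales length from those values.
; Pinch disables on second-finger release until the first lifts, working around an engine bug.
; Flick only computes a viewport-normalized direction vector from touch positions, with optional debug output.
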(event `Input Touch Pressed`
  (params (Location :type "Vector Structure") (`Finger Index` :type "ETouchIndex Enum" :default "Touch1"))
  ;[1 1 1] In the actor, this needs to be connected to touch for pressed and released with finger index
  ;[1 1 1] Is it multitouching?
  ;;[1 1 1] Used to determine flick strength
  (set `self.Touch pressed location` Location)
  (switch `ETouchIndex` `Finger Index`
    (:`Touch2`
      (bind (_spring_arm_component _spring_arm_world_rotation _targetarmlength) (`self.Get Springarm Node`))
      (set `self.Spring Arm Component` _spring_arm_component)
      (set `self.Spring Arm Starting Abs Rotation` _spring_arm_world_rotation)
      (set `self.Spring Arm Starting Target Arm Length` _targetarmlength))))

(event `Input Touch Released`
  (params (Location :type "Vector Structure") (`Finger Index` :type "ETouchIndex Enum" :default "Touch1"))
  ;[1 1 1] In the actor, this needs to be connected to touch for pressed and released with finger index
  ;[1 1 1] Is it multitouching?
  ;;[1 1 1] Used to determine flick strength
  (set `self.Touch released location` Location)
  (switch `ETouchIndex` `Finger Index`
    (:`Touch1`
      ;[1 1 1] Disable pinch when second finger is lifted until first finger is lifted. This is due to pinch bug.
      (set `self.Pinch Enabled` true))
    (:`Touch2`
      (set `self.Pinch Enabled` false))))

(event `Rotate Component`
  (params (AxisValue :type "Float (double-precision)"))
  (bind (_spring_arm_starting_abs_rotation_roll _spring_arm_starting_abs_rotation_pitch _spring_arm_starting_abs_rotation_yaw) (`KismetMathLibrary.BreakRotator` (`self.Spring Arm Starting Abs Rotation`)))
  ;[1 1 1] In project settings, create axis mapping for Gesture: rotate, pinch, and flick; then in player's actor, connect them to these these events
  ;;[1 1 1] Rotate
  ;;;[1 1 1] Axis value is rotation from initial rotation between finger positions
  (bind (_spring_arm_component _spring_arm_world_rotation) (`self.Get Springarm Node`))
  (`SceneComponent.K2_SetWorldRotation` _spring_arm_component (`KismetMathLibrary.RInterpTo` _spring_arm_world_rotation (`KismetMathLibrary.MakeRotator` (+ (* AxisValue -1.0) _spring_arm_starting_abs_rotation_roll) _spring_arm_starting_abs_rotation_pitch _spring_arm_starting_abs_rotation_yaw) (`GameplayStatics.GetWorldDeltaSeconds`) 100.0) false false))

(event `Pinch Component`
  (params (AxisValue :type "Float (double-precision)"))
  (bind _returnvalue (`KismetMathLibrary.FInterpTo` (`SpringArmComponent.TargetArmLength` (`self.Spring Arm Component`)) (* AxisValue (`self.Spring Arm Starting Target Arm Length`)) (`GameplayStatics.GetWorldDeltaSeconds`) 25.0))
  ;[1 1 1] In project settings, create axis mapping for Gesture: rotate, pinch, and flick; then in player's actor, connect them to these these events
  ;;[1 1 1] Pinch
  ;;;[1 1 1] Axis value is multiplier to initial pinch distance between fingers
  ;;;[1 1 1] Disables pinch unless both fingers have been lifted. There's a bug in UE4 that causes pinch component axis value to (Sometimes) not get reset to 1.0 when the second finger is lifted and then placed back before the first finger is lifted.
  (if (`self.Pinch Enabled`)
    (set `SpringArmComponent.TargetArmLength` _returnvalue (`self.Spring Arm Component`))
    (`self.Print String Label + Input Value` false "TargetArmLength" (`KismetStringLibrary.Conv_DoubleToString` _returnvalue))))

(event `Flick Component`
  (params (AxisValue :type "Float (double-precision)"))
  (bind (_returnvalue_x _returnvalue_y) (`KismetMathLibrary.BreakVector2D` (`WidgetLayoutLibrary.GetViewportSize`)))
  (bind (_returnvalue_x_2 _returnvalue_y_2) (`KismetMathLibrary.BreakVector2D` (`WidgetLayoutLibrary.GetViewportSize`)))
  (bind (_touch_pressed_location_x _touch_pressed_location_y) (`KismetMathLibrary.BreakVector` (`self.Touch pressed location`)))
  (bind (_touch_released_location_x _touch_released_location_y) (`KismetMathLibrary.BreakVector` (`self.Touch released location`)))
  (bind (_returnvalue_x_3 _returnvalue_y_3) (`KismetMathLibrary.BreakVector2D` (- (`KismetMathLibrary.MakeVector2D` (/ _touch_pressed_location_x _returnvalue_x_2) (/ _touch_pressed_location_y _returnvalue_y_2)) (`KismetMathLibrary.MakeVector2D` (/ _touch_released_location_x _returnvalue_x) (/ _touch_released_location_y _returnvalue_y)))))
  (bind (_returnvalue_x_4 _returnvalue_y_4) (`KismetMathLibrary.BreakVector` (* (`KismetMathLibrary.Conv_Vector2DToVector` (`self.Flick Direction Strength`)) 1000.0)))
  ;[1 1 1] In project settings, create axis mapping for Gesture: rotate, pinch, and flick; then in player's actor, connect them to these these events
  ;;[1 1 1] Flick
  (if (not (== AxisValue (`self.Last Flick Direction`)))
    (bind _output_get (set `self.Last Flick Direction` AxisValue))
    (`self.Print String Label + Input Value` false "Flick Direction " (`KismetStringLibrary.Conv_DoubleToString` _output_get))
    (set `self.Flick Direction Strength` (* (`KismetMathLibrary.MakeVector2D` _returnvalue_x_3 _returnvalue_y_3) (-1.0 1.0)))
    ;;[1 1 1] Debugging purposes
    (if false
      (`KismetSystemLibrary.DrawDebugLine` (0.0 0.0 0.0) (`KismetMathLibrary.MakeVector` 0.0 _returnvalue_x_4 _returnvalue_y_4) (struct :`R` 1.0 :`A` 1.0) 1.0 5.0)
      (`self.Print String Label + Input Value` false "Flick Direction Strength" (`KismetStringLibrary.Conv_Vector2dToString` (`self.Flick Direction Strength`)))
      (`self.Print String Label + Input Value` false "Touch pressed location" (`KismetStringLibrary.Conv_VectorToString` (`self.Touch pressed location`)))
      (`self.Print String Label + Input Value` false "Touch released location" (`KismetStringLibrary.Conv_VectorToString` (`self.Touch released location`))))))

(fn `Get Springarm Node`
  (returns (`Spring arm component` :type "SpringArmComponent Object Reference") (`Spring arm World Rotation` :type "Rotator Structure") (TargetArmLength :type "Float (double-precision)"))
  (bind _returnvalue (`Actor.GetComponentByClass` (`self.GetOwner`) "/Script/Engine.SpringArmComponent"))
  (return _returnvalue (`SceneComponent.K2_GetComponentRotation` _returnvalue) (`SpringArmComponent.TargetArmLength` _returnvalue)))

(fn `Is Finger Number True`
  (params (`Finger Index` :type Byte) (`Finger Index To Test To` :type Byte))
  (returns (`Finger index is equal` :type Boolean))
  (return (== `Finger Index` `Finger Index To Test To`)))

(fn `Print String Label + Input Value`
  (params (`Enable String Printing` :type Boolean) (Label :type String) (`String To Print` :type String))
  (if `Enable String Printing`
    (`KismetSystemLibrary.PrintString` (`KismetStringLibrary.Concat_StrStr` Label `String To Print`))))
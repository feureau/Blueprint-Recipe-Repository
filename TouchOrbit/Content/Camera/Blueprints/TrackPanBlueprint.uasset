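; Camera rig actor that pans and dollies a cine camera from touch, mouse and pinch input, with screen fades for resets.
; Each tick smooths pinch and, when panning is allowed, offsets the actor relative to motion controller rotation.
; The camera follows the controller's position above a minimum height.
; Timelines drive a fade-sphere dynamic material; orbit-ring setup is disconnected, and timer-updated drift direction goes unread here.
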(event `FadeUp`
  (`MaterialInstanceDynamic.SetScalarParameterValue` (`self.FadeMat`) "Fade" 1.0)
  (`SceneComponent.SetVisibility` (`self.FadeSphere`) true false)
  (bind (_direction _newtrack_0) (`Timeline|FadeUpTrack`)
    (:`Update`
      (`MaterialInstanceDynamic.SetScalarParameterValue` (`self.FadeMat`) "Fade" _newtrack_0))
    (:`Finished`
      (`SceneComponent.SetVisibility` (`self.FadeSphere`) false false))))

(event `FadeToReset`
  ;[1 1 1] Fade on Restart
  (`SceneComponent.SetVisibility` (`self.FadeSphere`) true false)
  (bind (_direction _fadetrack) (`Timeline|FadeTimer` :!via `PlayFromStart`)
    (:`Update`
      (`MaterialInstanceDynamic.SetScalarParameterValue` (`self.FadeMat`) "Fade" _fadetrack))
    (:`Finished`
      (`self.DoneFade`))))

(event `self.ReceiveTick`
  (params (DeltaSeconds :type "Float (single-precision)"))
  (bind _z (.z (`SceneComponent.K2_GetComponentLocation` (`self.MotionController`))))
  ;[1 1 1] Interaction controls
  (set `self.TickTime` DeltaSeconds)
  (bind _output_get (set `self.SmoothPinch` (`KismetMathLibrary.FInterpTo` (`self.SmoothPinch`) (`self.PinchInput`) (`self.TickTime`) (`KismetMathLibrary.SelectFloat` 10.0 25.0 (`self.Pinch`)))))
  (bind _returnvalue (`KismetMathLibrary.FClamp` (+ (* _output_get -2.0) (`self.FinalPinch`)) -600.0 600.0))
  (set `self.FinalPinch` (`KismetMathLibrary.SelectFloat` _returnvalue (`KismetMathLibrary.FInterpTo` _returnvalue 0.0 (`self.TickTime`) 0.125) (`self.Pinch`)))
  (if (`self.bAllowPanTrack`)
    (set `self.PitchAngle` (* (+ (`self.Mouse Y`) (`self.Touch Y`)) (`self.Y Touch Sensitivity`)))
    (`|ExecutionSequence`
      (:`then_0`
        (set `self.PitchAngle` (* (+ (`self.Mouse Y`) (`self.Touch Y`)) (`self.Y Touch Sensitivity`))))
      (:`then_1`
        (set `self.YawValue` (* (+ (`self.Touch X`) (`self.Mouse X`)) (`self.X Touch Sensitivity`))))
      (:`then_2`
        (`self.K2_AddActorLocalOffset` (`KismetMathLibrary.GreaterGreater_VectorRotator` (`KismetMathLibrary.VInterpTo` (`KismetMathLibrary.MakeVector` (`self.FinalPinch`) (- 0.0 (`self.YawValue`)) (- 0.0 (`self.PitchAngle`))) (0.0 0.0 0.0) (`self.TickTime`) 3.0) (`SceneComponent.RelativeRotation` (`self.MotionController`))))
        (`SceneComponent.K2_SetWorldLocation` (`self.CineCamera`) (`KismetMathLibrary.MakeVector` (.x (`SceneComponent.K2_GetComponentLocation` (`self.MotionController`))) (.y (`SceneComponent.K2_GetComponentLocation` (`self.MotionController`))) (`KismetMathLibrary.FClamp` _z 35.0 _z)) false false)))))

(event `ResetLoc`
  (`self.K2_SetActorLocation` (`self.SourceLoc`)))

(event `self.ReceiveBeginPlay`
  ;[1 1 1] Loop to update drift velocities
  (`KismetSystemLibrary.K2_SetTimerDelegate` (delegate `DriftChoice`) 0.05 true)
  (`KismetSystemLibrary.K2_SetTimer` null "CustomTick" 0.05 true))

(event `DriftChoice`
  (bind _returnvalue (+ (`self.Mouse X`) (`self.Touch X`)))
  ;[1 1 1] Loop to update drift velocities
  (if (> _returnvalue 0.005)
    (set `self.Drift Amount` 0.02)
    (elif (< _returnvalue -0.005)
      (set `self.Drift Amount` -0.02))))

(fn `FadeComplete`)

(fn `UserConstructionScript`
  (`CameraComponent.SetFieldOfView` (`self.CineCamera`) (`self.Orbit FOV`))
  (bind _returnvalue (`PrimitiveComponent.CreateDynamicMaterialInstance` (`self.FadeSphere`) 0 "/Game/Camera/Effects/Materials/M_CameraFade.M_CameraFade" "None"))
  (set `self.FadeMat` _returnvalue))
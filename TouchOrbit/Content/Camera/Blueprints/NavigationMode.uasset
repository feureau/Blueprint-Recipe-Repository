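; Navigation mode Blueprint that switches camera states between startup, orbit and two interactions through a StateChange event.
; Orbit blends the player view to OrbitClass, enables orbiting and eases in drift with a timeline, skipping this when returning from power.
; Both interactions set a blend time and re-enter Orbit; PowerMode or the J key triggers the second from orbit, while the first's trigger is unwired.
; SwapModel only stores a model index.
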(event `SwapModel`
  (params (Index :type Integer))
  (set `self.ModelIndex` Index))

(event `StateChange`
  (params (NewState :type "/Game/Camera/Blueprints/DemoState Enum" :default "NewEnumerator0"))
  (bind _orbitclass (`self.OrbitClass`))
  ;[1 1 1] Handle State Changes
  (switch `/Game/Camera/Blueprints/DemoState` NewState
    (:`NewEnumerator0`
      (set `self.bInOrbitState` false)
      (set `/Game/Camera/Blueprints/OrbitBlueprint.bAllowOrbit` false _orbitclass)
      (set `/Game/Camera/Blueprints/OrbitBlueprint.Drift Amount` 0.0 _orbitclass)
      (set `self.TransitionTime` 0.2))
    (:`NewEnumerator1`
      (set `self.bInOrbitState` true)
      (if (`self.bComingFromPower`)
        (set `self.bComingFromPower` false)
        (else
          (set `/Game/Camera/Blueprints/OrbitBlueprint.bAllowOrbit` true (`self.OrbitClass`))
          (`PlayerController.SetViewTargetWithBlend` (`GameplayStatics.GetPlayerController` 0) (`self.OrbitClass`) (`self.TransitionTime`) "VTBlend_Linear" 0.0 false)
          (bind (_direction _interp_weighting) (`Timeline|Timeline_0` :!via `PlayFromStart`)
            (:`Update`
              (set `/Game/Camera/Blueprints/OrbitBlueprint.Drift Amount` (`KismetMathLibrary.Lerp` 0.0 -0.08 _interp_weighting) (`self.OrbitClass`)))))))
    (:`NewEnumerator2`
      (set `/Game/Camera/Blueprints/OrbitBlueprint.YawValue` -3.0 (`self.OrbitClass`))
      (set `self.TransitionTime` 1.5)
      (`self.StateChange` "NewEnumerator1"))
    (:`NewEnumerator3`
      (set `self.TransitionTime` 1.0)
      (`self.StateChange` "NewEnumerator1"))))

(event `PowerMode`
  (if (`self.bInOrbitState`) :!label _label
    (`self.StateChange` "NewEnumerator3")))

(event `Key|J`
  (params (Key :type "Key Structure"))
  (:`Pressed`
    (goto _label)))

(fn `UserConstructionScript`)